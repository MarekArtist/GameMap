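; BP_ChangeMap is a trigger box actor that switches the player's minimap style when the player's ThirdPersonCharacter overlaps it.
; Flags select 3D, 2D or a shape change.
; The 3D and 2D modes swap the widget's image brush and toggle the 3DMinimap scene capture, with 3D also putting the AutoMap material on its plane.
; Otherwise it sets the material's rectangular or circular parameter and regenerates the widget's shape.
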(event `self.Box.OnComponentBeginOverlap`
  (params (OverlappedComponent :type "PrimitiveComponent Object Reference") (OtherActor :type "Actor Object Reference") (OtherComp :type "PrimitiveComponent Object Reference") (OtherBodyIndex :type Integer) (bFromSweep :type Boolean) (SweepResult :type "HitResult Structure (by ref)"))
  (bind _3d_minimap (`self.3D minimap`))
  (if (and (== OtherActor (`GameplayStatics.GetPlayerPawn` 0)) (!= (`GameplayStatics.GetObjectClass` OtherComp) "/Script/Engine.BoxComponent"))
    (bind _asthird_person_character (cast `/Game/UltraMap/Mannequin/Character/ThirdPersonCharacter` (`GameplayStatics.GetPlayerPawn` 0))
      (:`then`
        (`/Engine/EditorBlueprintResources/StandardMacros.IsValid` (`/Game/UltraMap/Mannequin/Character/ThirdPersonCharacter.Minimap` _asthird_person_character)
          (:`Is Valid`
            (if (`self.3D?`)
              (bind _minimap (`/Game/UltraMap/Mannequin/Character/ThirdPersonCharacter.Minimap` _asthird_person_character))
              (bind _imagerender (`/Game/UltraMap/UltraMap/WBP_UltraMap.ImageRender` _minimap))
              (bind (_brush_imagesize _brush_drawas _brush_margin _brush_tintcolor _brush_tiling _brush_mirroring) (break `SlateBrush` (`Image.Brush` _imagerender)))
              (`Image.SetBrush` _imagerender (make `SlateBrush` _brush_imagesize _brush_drawas _brush_margin _brush_tintcolor _brush_tiling _brush_mirroring "/Game/UltraMap/UltraMap/graphics/Rendering/3D_Minimap/MAT_MinimapCapture.MAT_MinimapCapture")) ; replace AutoMap with 3DMinimapMaterial
              (set `/Game/UltraMap/UltraMap/graphics/Rendering/3D_Minimap/BP_minimapCapture.Turn on` true _3d_minimap) ; turn ON scene capture component
              (`PrimitiveComponent.SetMaterial` (`/Game/UltraMap/UltraMap/graphics/Rendering/3D_Minimap/BP_minimapCapture.Plane` _3d_minimap) 0 (`/Game/UltraMap/UltraMap/WBP_UltraMap.AutoMapInstance` _minimap)) ; use AutoMap material for scene capture
              (elif (`self.2D?`)
                (bind _minimap_2 (`/Game/UltraMap/Mannequin/Character/ThirdPersonCharacter.Minimap` _asthird_person_character))
                (bind _imagerender_2 (`/Game/UltraMap/UltraMap/WBP_UltraMap.ImageRender` _minimap_2))
                (bind (_brush_imagesize_2 _brush_drawas_2 _brush_margin_2 _brush_tintcolor_2 _brush_tiling_2 _brush_mirroring_2) (break `SlateBrush` (`Image.Brush` _imagerender_2)))
                (`Image.SetBrush` _imagerender_2 (make `SlateBrush` _brush_imagesize_2 _brush_drawas_2 _brush_margin_2 _brush_tintcolor_2 _brush_tiling_2 _brush_mirroring_2 (`/Game/UltraMap/UltraMap/WBP_UltraMap.AutoMapInstance` _minimap_2))) ; reverse
                (set `/Game/UltraMap/UltraMap/graphics/Rendering/3D_Minimap/BP_minimapCapture.Turn on` false _3d_minimap) ; turn OFF scene capture component if not needed
                (else
                  (if (`self.Rectangular`)
                    (bind _automapinstance (`/Game/UltraMap/UltraMap/WBP_UltraMap.AutoMapInstance` _minimap_2))
                    (`MaterialInstanceDynamic.SetScalarParameterValue` _automapinstance "Rectangular/Circular" 0.0) ; switch shape rendering in AutoMap material
                    (set `/Game/UltraMap/UltraMap/WBP_UltraMap.shape` 1 _minimap_2) ; swtich shape in intersection checks in UltraMap widget
                    (else
                      (`MaterialInstanceDynamic.SetScalarParameterValue` _automapinstance "Rectangular/Circular" 1.0)
                      (set `/Game/UltraMap/UltraMap/WBP_UltraMap.shape` 0 _minimap_2)))
                  (`/Game/UltraMap/UltraMap/WBP_UltraMap.Set shape` _minimap_2) ; generate vertices
                ))))))
      (:`CastFailed`
        (`KismetSystemLibrary.PrintString` "Minimap could not be changed (Cast to ThirdPerson fail)")))))

(fn `UserConstructionScript`)