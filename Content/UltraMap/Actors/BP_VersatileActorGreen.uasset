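; BP_VersatileActorGreen is a clickable actor that switches between being a local and a global point on the UltraMap minimap.
; Clicking it toggles Blink, adding or removing its global point and updating the local registration through the map reference passed in.
; While it blinks, overlap events remove its local point.
; The construction script builds a dynamic blinking material with configurable colors, whose Blink parameter mirrors the toggle.
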(event `/Game/UltraMap/UltraMap/BI_MinimapInterface.StartOverlap`
  (params (`Minimap reference` :type "/Game/UltraMap/UltraMap/WBP_UltraMap Object Reference"))
  (if (`self.Blink?`)
    (`/Game/UltraMap/UltraMap/WBP_UltraMap.RemoveLocal` `Minimap reference` self)))

(event `/Game/UltraMap/UltraMap/BI_MinimapInterface.ActorClick`
  (params (Actor :type "Actor Object Reference") (Umap :type "/Game/UltraMap/UltraMap/WBP_UltraMap Object Reference"))
  (bind _upoint_class (`self.Upoint class`))
  (if (== Actor self)
    (if (`self.Blink?`)
      (`/Game/UltraMap/UltraMap/WBP_UltraMap.Global point` Umap self _upoint_class true)
      (set `self.Blink?` false)
      (`MaterialInstanceDynamic.SetScalarParameterValue` (`self.MyMaterial`) "Blink?" (`KismetMathLibrary.Conv_IntToDouble` (`KismetMathLibrary.Conv_BoolToInt` (`self.Blink?`))))
      (`KismetSystemLibrary.Delay` 0.2)
      (`/Game/UltraMap/UltraMap/WBP_UltraMap.Begin overlap` Umap self)
      (else
        (`/Game/UltraMap/UltraMap/WBP_UltraMap.RemoveLocal` Umap self)
        (`/Game/UltraMap/UltraMap/WBP_UltraMap.Recognize points` Umap (`GameplayStatics.GetObjectClass` self) _upoint_class null true)
        (`/Game/UltraMap/UltraMap/WBP_UltraMap.Global point` Umap self null false)
        (set `self.Blink?` true)
        (`MaterialInstanceDynamic.SetScalarParameterValue` (`self.MyMaterial`) "Blink?" (`KismetMathLibrary.Conv_IntToDouble` (`KismetMathLibrary.Conv_BoolToInt` (`self.Blink?`))))))))

(fn `UserConstructionScript`
  (bind _returnvalue (`KismetMaterialLibrary.CreateDynamicMaterialInstance` "/Game/UltraMap/Materials/MAT_Blinking.MAT_Blinking"))
  (bind _output_get (set `self.MyMaterial` _returnvalue))
  (`MaterialInstanceDynamic.SetVectorParameterValue` _output_get "BaseColor" (`self.BaseColor`))
  (`MaterialInstanceDynamic.SetVectorParameterValue` _output_get "BlinkColor" (`self.BlinkColor`))
  (`MaterialInstanceDynamic.SetScalarParameterValue` _output_get "Blink?" (`KismetMathLibrary.Conv_IntToDouble` (`KismetMathLibrary.Conv_BoolToInt` (`self.Blink?`))))
  (`PrimitiveComponent.SetMaterial` (`self.Me`) 0 (`self.MyMaterial`)))