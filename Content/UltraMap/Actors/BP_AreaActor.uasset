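; BP_AreaActor is a map area for the UltraMap minimap that changes its look when the player enters.
; StartOverlap stores the minimap reference and sends it an original-colored dynamic material, or the changed one if StayChanged has latched.
; The box overlap filters for the player pawn, ignoring its box components, then sends a changed-color material through ChangeArea.
; WasChanged blocks repeat changes and resets immediately unless StayChanged is set.
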(event `/Game/UltraMap/UltraMap/BI_MinimapInterface.StartOverlap`
  (params (`Minimap reference` :type "/Game/UltraMap/UltraMap/WBP_UltraMap Object Reference"))
  (set `self.Minimap` `Minimap reference`)
  (if (and (`self.wasChanged?`) (`self.Stay changed?`))
    (`/Game/UltraMap/UltraMap/WBP_UltraMap.Change Area` (`self.Minimap`) self (stale `self.Box.OnComponentBeginOverlap` _returnvalue) :!label _label) ; call UltraMap
    (if (not (`self.Stay changed?`))
      (set `self.wasChanged?` false))
    (else
      (bind _returnvalue (`KismetMaterialLibrary.CreateDynamicMaterialInstance` (`self.Original Material`)))
      (`MaterialInstanceDynamic.SetVectorParameterValue` _returnvalue "foreground" (`self.Fore color`))
      (`MaterialInstanceDynamic.SetVectorParameterValue` _returnvalue "background" (`self.Back color`))
      (`/Game/UltraMap/UltraMap/WBP_UltraMap.Change Area` (`self.Minimap`) self _returnvalue) ; call UltraMap
    )))

(event `self.Box.OnComponentBeginOverlap`
  (params (OverlappedComponent :type "PrimitiveComponent Object Reference") (OtherActor :type "Actor Object Reference") (OtherComp :type "PrimitiveComponent Object Reference") (OtherBodyIndex :type Integer) (bFromSweep :type Boolean) (SweepResult :type "HitResult Structure (by ref)"))
  ;[1 1 1] is player in?
  (if (and (== OtherActor (`GameplayStatics.GetPlayerPawn` 0)) (!= (`GameplayStatics.GetObjectClass` OtherComp) "/Script/Engine.BoxComponent"))
    (if (not (`self.wasChanged?`))
      (set `self.wasChanged?` true)
      (bind _returnvalue (`KismetMaterialLibrary.CreateDynamicMaterialInstance` (`self.Changed material`)))
      (`MaterialInstanceDynamic.SetVectorParameterValue` _returnvalue "foreground" (`self.Fore color changed`))
      (`MaterialInstanceDynamic.SetVectorParameterValue` _returnvalue "background" (`self.Back color changed`))
      (goto _label))))

(fn `UserConstructionScript`)