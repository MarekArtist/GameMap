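; BP_PointGateGlobal is a trigger volume that changes which actors show as global points on the player's minimap.
; When the player pawn overlaps its box, excluding overlapping box components, it sends each listed actor to the ThirdPersonCharacter's Minimap.
; Parallel arrays supply each actor's Upoint render class and whether that point is added or removed.
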(event `self.Box.OnComponentBeginOverlap`
  (params (OverlappedComponent :type "PrimitiveComponent Object Reference") (OtherActor :type "Actor Object Reference") (OtherComp :type "PrimitiveComponent Object Reference") (OtherBodyIndex :type Integer) (bFromSweep :type Boolean) (SweepResult :type "HitResult Structure (by ref)"))
  (bind _returnvalue (`GameplayStatics.GetPlayerPawn` 0))
  ;[1 1 1] Is player in?
  (if (and (== OtherActor _returnvalue) (!= (`GameplayStatics.GetObjectClass` OtherComp) "/Script/Engine.BoxComponent"))
    (bind _asthird_person_character (cast `/Game/UltraMap/Mannequin/Character/ThirdPersonCharacter` _returnvalue))
    (`/Engine/EditorBlueprintResources/StandardMacros.IsValid` (`/Game/UltraMap/Mannequin/Character/ThirdPersonCharacter.Minimap` _asthird_person_character)
      (:`Is Valid`
        (for (_array_element _array_index) (`self.Actors concerned`)
          (message `/Game/UltraMap/UltraMap/BI_MinimapInterface.Global point` (`/Game/UltraMap/Mannequin/Character/ThirdPersonCharacter.Minimap` _asthird_person_character) _array_element (`|GetArrayItem` (`self.Upoint classes`) _array_index) (`|GetArrayItem` (`self.Remove?`) _array_index)))))))

(fn `UserConstructionScript`)