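; BP_PointGateLocal is a trigger gate that changes which actor classes the local player's minimap recognizes as points.
; When player pawn 0 overlaps its Box with a non-box component, it reaches the Minimap through ThirdPersonCharacter.
; It loops over ActorClasses, using the parallel StopRecognizing flags to stop or start recognition per class.
; Started classes all receive the first UpointClasses entry, whatever their index.
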(event `self.Box.OnComponentBeginOverlap`
  (params (OverlappedComponent :type "PrimitiveComponent Object Reference") (OtherActor :type "Actor Object Reference") (OtherComp :type "PrimitiveComponent Object Reference") (OtherBodyIndex :type Integer) (bFromSweep :type Boolean) (SweepResult :type "HitResult Structure (by ref)"))
  (bind _returnvalue (`GameplayStatics.GetPlayerPawn` 0))
  ;[1 1 1] Is player in
  (if (and (== OtherActor _returnvalue) (!= (`GameplayStatics.GetObjectClass` OtherComp) "/Script/Engine.BoxComponent"))
    (bind _asthird_person_character (cast `/Game/UltraMap/Mannequin/Character/ThirdPersonCharacter` _returnvalue)
      (:`then`
        (`/Engine/EditorBlueprintResources/StandardMacros.IsValid` (`/Game/UltraMap/Mannequin/Character/ThirdPersonCharacter.Minimap` _asthird_person_character)
          (:`Is Valid`
            (for (_array_element _array_index) (`self.Actor classes`)
              (if (`|GetArrayItem` (`self.Stop recognizing?`) _array_index)
                (bind _minimap (`/Game/UltraMap/Mannequin/Character/ThirdPersonCharacter.Minimap` _asthird_person_character))
                (`/Game/UltraMap/UltraMap/WBP_UltraMap.Stop recognizing` _minimap _array_element)
                (else
                  (`/Game/UltraMap/UltraMap/WBP_UltraMap.Recognize points` _minimap _array_element (`|GetArrayItem` (`self.Upoint classes`)) null false)))))
          (:`Is Not Valid`
            (`KismetSystemLibrary.PrintString` "Minimap not found in ThirdPersonCharacter" true true (struct :`R` 1.0 :`B` 0.106452 :`A` 1.0)))))
      (:`CastFailed`
        (`KismetSystemLibrary.PrintString` "Cast to ThirdPersonCharacter FAILED" true true (struct :`R` 1.0 :`B` 0.013641 :`A` 1.0))))))

(fn `UserConstructionScript`)