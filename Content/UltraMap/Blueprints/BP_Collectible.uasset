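; BP_Collectible is an UltraMap collectible that tracks player proximity and can be removed from the map.
; Its trigger box, scaled from the mesh in construction, sets InRange and registers or clears the collectible as InRangeActor on ThirdPersonCharacter, ignoring box components.
; StartOverlap stores the minimap reference.
; ActorClick destroys the collectible when its map point is clicked, with no range check.
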(event `/Game/UltraMap/UltraMap/BI_MinimapInterface.StartOverlap`
  (params (`Minimap reference` :type "/Game/UltraMap/UltraMap/WBP_UltraMap Object Reference"))
  ;[1 1 1] Store minimap's reference
  (set `self.Minimap` `Minimap reference`))

(event `self.Box.OnComponentBeginOverlap`
  (params (OverlappedComponent :type "PrimitiveComponent Object Reference") (OtherActor :type "Actor Object Reference") (OtherComp :type "PrimitiveComponent Object Reference") (OtherBodyIndex :type Integer) (bFromSweep :type Boolean) (SweepResult :type "HitResult Structure (by ref)"))
  (bind _returnvalue (`GameplayStatics.GetPlayerCharacter` 0))
  ;[1 1 1] Is it player who is close (and not its collision box)
  (if (!= (`GameplayStatics.GetObjectClass` OtherComp) "/Script/Engine.BoxComponent")
    (if (== OtherActor _returnvalue)
      (set `self.inRange` true)
      (bind _asthird_person_character (cast `/Game/UltraMap/Mannequin/Character/ThirdPersonCharacter` _returnvalue)
        (:`then`
          ;[1 1 1] stores itself to the memory inside character BP
          (set `/Game/UltraMap/Mannequin/Character/ThirdPersonCharacter.inRangeActor` self _asthird_person_character))
        (:`CastFailed`
          (`KismetSystemLibrary.PrintString` "Cannot affect item (Cast to ThirdPersonCharacter failed)" :!label _label))))))

(event `self.Box.OnComponentEndOverlap`
  (params (OverlappedComponent :type "PrimitiveComponent Object Reference") (OtherActor :type "Actor Object Reference") (OtherComp :type "PrimitiveComponent Object Reference") (OtherBodyIndex :type Integer))
  (bind _returnvalue (`GameplayStatics.GetPlayerCharacter` 0))
  ;[1 1 1] Is it player who is close (and not its collision box)
  (if (!= (`GameplayStatics.GetObjectClass` OtherComp) "/Script/Engine.BoxComponent")
    (if (== OtherActor _returnvalue)
      (set `self.inRange` false)
      (bind _asthird_person_character (cast `/Game/UltraMap/Mannequin/Character/ThirdPersonCharacter` _returnvalue)
        (:`then`
          (if (== (`/Game/UltraMap/Mannequin/Character/ThirdPersonCharacter.inRangeActor` _asthird_person_character) self)
            ;[1 1 1] removes  itself from  the memory inside character BP
            (set `/Game/UltraMap/Mannequin/Character/ThirdPersonCharacter.inRangeActor` null _asthird_person_character)))
        (:`CastFailed`
          (goto _label))))))

(event `/Game/UltraMap/UltraMap/BI_MinimapInterface.ActorClick`
  (params (Actor :type "Actor Object Reference") (Umap :type "/Game/UltraMap/UltraMap/WBP_UltraMap Object Reference"))
  ;[1 1 1] Destroy self when UltraMap says that player clicked on its point
  (if (== Actor self)
    (`self.K2_DestroyActor` Actor)))

(fn `UserConstructionScript`
  (`SceneComponent.SetRelativeScale3D` (`self.Box`) (* (`SceneComponent.RelativeScale3D` (`self.StaticMeshComponent0`)) 5.0)))