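; Automatic sliding double door that opens with sound when the player pawn enters its trigger box and closes on exit, ignoring overlaps from box components.
; MoveComponentTo slides both panels apart or together, while an InAction counter blocks retriggering mid-move and PlayerIn tracks the open state.
; The construction script gives both sensors one dynamic material for colored state display and enables or disables the trigger via Onoff.
; BeginOpen opens it at BeginPlay.
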(event `CloseLeft`
  (bind _doorleft (`self.doorLeft`))
  ;[1 0 0.01632] Door Closure
  (`KismetSystemLibrary.MoveComponentTo` _doorleft (+ (`SceneComponent.RelativeLocation` _doorleft) (70.0 0.0 0.0)) (`SceneComponent.RelativeRotation` _doorleft) true true 0.5)
  (set `self.inAction` (- (`self.inAction`) 1))
  (set `self.PlayerIn` false))

(event `Close`
  ;[1 0.01504 0] Close the door and change the material parameter
  (if (not (> (`self.inAction`) 0))
    (set `self.inAction` 2)
    (`self.CloseRight`)
    (`self.CloseLeft`)
    (`MaterialInstanceDynamic.SetScalarParameterValue` (`self.SensorMat`) "State" 0.0)))

(event `CloseRight`
  (bind _doorright (`self.doorRight`))
  ;[1 0 0.01632] Door Closure
  (`KismetSystemLibrary.MoveComponentTo` _doorright (- (`SceneComponent.RelativeLocation` _doorright) (70.0 0.0 0.0)) (`SceneComponent.RelativeRotation` _doorright) true true 0.5)
  (set `self.inAction` (- (`self.inAction`) 1)))

(event `OpenLeft`
  (bind _doorleft (`self.doorLeft`))
  ;[0 1 0.2004] Door Opening
  (`KismetSystemLibrary.MoveComponentTo` _doorleft (- (`SceneComponent.RelativeLocation` _doorleft) (70.0 0.0 0.0)) (`SceneComponent.RelativeRotation` _doorleft) true true 0.5)
  (set `self.inAction` (- (`self.inAction`) 1))
  (set `self.PlayerIn` true))

(event `Open`
  ;[0 1 0.003698] Open the door and change the material parameter to "open"
  (if (not (> (`self.inAction`) 0))
    (set `self.inAction` 2)
    (`self.OpenRight`)
    (`self.OpenLeft`)
    (`MaterialInstanceDynamic.SetScalarParameterValue` (`self.SensorMat`) "State" 1.0)))

(event `OpenRight`
  (bind _doorright (`self.doorRight`))
  ;[0 1 0.2004] Door Opening
  (`KismetSystemLibrary.MoveComponentTo` _doorright (+ (`SceneComponent.RelativeLocation` _doorright) (70.0 0.0 0.0)) (`SceneComponent.RelativeRotation` _doorright) true true 0.5)
  (set `self.inAction` (- (`self.inAction`) 1)))

(event `self.ReceiveBeginPlay`
  ;[1 1 1] Should door be open from the beginning?
  (if (`self.Begin open`)
    (set `self.PlayerIn` true)
    (`self.Open`)))

(event `self.Box.OnComponentBeginOverlap`
  (params (OverlappedComponent :type "PrimitiveComponent Object Reference") (OtherActor :type "Actor Object Reference") (OtherComp :type "PrimitiveComponent Object Reference") (OtherBodyIndex :type Integer) (bFromSweep :type Boolean) (SweepResult :type "HitResult Structure (by ref)"))
  (bind _returnvalue (`self.K2_GetActorLocation`))
  ;[0.4921 0.784 1] "Motion sensor"
  (if (!= (`GameplayStatics.GetObjectClass` OtherComp) "/Script/Engine.BoxComponent")
    (if (`self.PlayerIn`)
      _
      (elif (== OtherActor (`GameplayStatics.GetPlayerPawn` 0))
        (`GameplayStatics.PlaySoundAtLocation` "/Game/UltraMap/Audio/Cues/CUE_DoorActivation.CUE_DoorActivation" _returnvalue)
        (`GameplayStatics.PlaySoundAtLocation` "/Game/UltraMap/Audio/Cues/CUE_Door.CUE_Door" _returnvalue) ; opening sound
        (`self.Open`) ; Open if not opened
      ))))

(event `self.Box.OnComponentEndOverlap`
  (params (OverlappedComponent :type "PrimitiveComponent Object Reference") (OtherActor :type "Actor Object Reference") (OtherComp :type "PrimitiveComponent Object Reference") (OtherBodyIndex :type Integer))
  ;[0.4921 0.784 1] "Motion sensor"
  (if (!= (`GameplayStatics.GetObjectClass` OtherComp) "/Script/Engine.BoxComponent")
    (if (`self.PlayerIn`)
      (if (== (`GameplayStatics.GetPlayerPawn` 0) OtherActor)
        (`GameplayStatics.PlaySoundAtLocation` "/Game/UltraMap/Audio/Cues/CUE_DoorClose.CUE_DoorClose" (`self.K2_GetActorLocation`)) ; closing sound
        (`self.Close`) ; Close if not closed
      ))))

(fn `UserConstructionScript`
  (bind _box (`self.Box`))
  (`|ExecutionSequence`
    (:`then_0`
      (bind _returnvalue (`PrimitiveComponent.CreateDynamicMaterialInstance` (`self.sensor`) 0 "/Game/UltraMap/Materials/MAT_SensorMat.MAT_SensorMat"))
      (bind _output_get (set `self.SensorMat` _returnvalue))
      (`MaterialInstanceDynamic.SetVectorParameterValue` _output_get "LockedColor" (`self.LockedColor`))
      (`MaterialInstanceDynamic.SetVectorParameterValue` _output_get "OpenColor" (`self.OpenColor`))
      (`MaterialInstanceDynamic.SetVectorParameterValue` _output_get "ClosedColor" (`self.ClosedColor`))
      (`MaterialInstanceDynamic.SetScalarParameterValue` _output_get "State" (`KismetMathLibrary.Conv_IntToDouble` (`self.Initial State`)))
      (`MaterialInstanceDynamic.SetScalarParameterValue` _output_get "LightIntensity" (`self.LightIntensity`))
      (if (`self.On/off`)
        (`PrimitiveComponent.SetCollisionEnabled` _box "QueryAndPhysics")
        (else
          (`PrimitiveComponent.SetCollisionEnabled` _box "NoCollision"))))
    (:`then_1`
      (`PrimitiveComponent.SetMaterial` (`self.sensor2`) 0 (`self.SensorMat`)))))