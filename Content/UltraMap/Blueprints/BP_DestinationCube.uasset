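; BP_DestinationCube is a clickable world actor that serves as a navigation destination for the UltraMap minimap.
; When clicked, it computes a synchronous navmesh path from the player pawn to itself and, if one exists, sends it to the map via SetPath.
; It then sets itself as ActorToFollow on the map's BP_MessageListener so the path can be re-found if not followed, printing a warning if that listener cast fails.
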(event `/Game/UltraMap/UltraMap/BI_MinimapInterface.ActorClick`
  (params (Actor :type "Actor Object Reference") (Umap :type "/Game/UltraMap/UltraMap/WBP_UltraMap Object Reference"))
  (if (== Actor self)
    (bind _returnvalue (`NavigationSystem.FindPathToActorSynchronously` (`self.K2_GetActorLocation` (`GameplayStatics.GetPlayerPawn` 0)) self))
    (if (> (`NavigationPath.GetPathLength` _returnvalue) 0.0)
      ;[1 1 1] Send path to minimap
      (`/Game/UltraMap/UltraMap/WBP_UltraMap.Set path` Umap _returnvalue)
      ;[1 1 1] Enables message listener to find new path if this one is not being followed
      (bind _asbp_message_listener (cast `/Game/UltraMap/Blueprints/BP_MessageListener` (`/Game/UltraMap/UltraMap/WBP_UltraMap.Listener` Umap))
        (:`then`
          (set `/Game/UltraMap/Blueprints/BP_MessageListener.ActorToFollow` self _asbp_message_listener))
        (:`CastFailed`
          (`KismetSystemLibrary.PrintString` "Destination cube could not reach the default message listener \"BP_MessageListener\"" true true (struct :`G` 0.66 :`B` 1.0 :`A` 1.0) 5.0))))))

(fn `UserConstructionScript`)