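; Interactive stand that lets the player pick up the item on it or place a carried one, keeping the UltraMap minimap informed of placed items.
; Box overlap tracks player proximity and registers the stand as the character's InRangeActor.
; When the player is close, Action either stores ItemAbove's class in GrabbedItem and destroys it, or spawns that class at the Plane, notifies the Minimap and clears GrabbedItem.
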(event `Action`
  (params (player :type "Pawn Object Reference"))
  ;[1 1 1] GRAB or PLACE
  (if (and (`self.playerClose?`) (`KismetSystemLibrary.IsValid` player))
    (bind _asthird_person_character (cast `/Game/UltraMap/Mannequin/Character/ThirdPersonCharacter` player)
      (:`then`
        (if (`KismetSystemLibrary.IsValidClass` (`/Game/UltraMap/Mannequin/Character/ThirdPersonCharacter.grabbedItem` _asthird_person_character))
          (bind _returnvalue (`|SpawnActorFromClass` (`/Game/UltraMap/Mannequin/Character/ThirdPersonCharacter.grabbedItem` _asthird_person_character) (`KismetMathLibrary.MakeTransform` (`SceneComponent.K2_GetComponentLocation` (`self.Plane`)) (struct) (0.4 0.5 0.2)) "AdjustIfPossibleButAlwaysSpawn" "OverrideRootScale")) ; Spawns actor that was until now in the "inventory"
          (bind _output_get (set `self.ItemAbove` _returnvalue))
          (`/Game/UltraMap/UltraMap/WBP_UltraMap.Begin overlap` (`/Game/UltraMap/Mannequin/Character/ThirdPersonCharacter.Minimap` _asthird_person_character) _output_get) ; Informs Ultra Map about new actor placed near the player
          (set `/Game/UltraMap/Mannequin/Character/ThirdPersonCharacter.grabbedItem` null _asthird_person_character) ; Removes item from "inventory"
          (else
            (set `/Game/UltraMap/Mannequin/Character/ThirdPersonCharacter.grabbedItem` (`GameplayStatics.GetObjectClass` (`self.ItemAbove`)) _asthird_person_character) ; Adds item to "inventory"
            (`/Engine/EditorBlueprintResources/StandardMacros.IsValid` (`self.ItemAbove`)
              (:`Is Valid`
                (`self.K2_DestroyActor` (`self.ItemAbove`)) ; Removes item from the world
              )))))
      (:`CastFailed`
        (`KismetSystemLibrary.PrintString` "Cast to ThirdPersonCharacter failed. Did you change the player pawn/character?")))))

(event `self.Box.OnComponentBeginOverlap`
  (params (OverlappedComponent :type "PrimitiveComponent Object Reference") (OtherActor :type "Actor Object Reference") (OtherComp :type "PrimitiveComponent Object Reference") (OtherBodyIndex :type Integer) (bFromSweep :type Boolean) (SweepResult :type "HitResult Structure (by ref)"))
  ;[1 1 1] Stores the actor placed on the stand to memory (as a nearby actor) AND detect if player is close enough
  (if (and (== OtherActor (`GameplayStatics.GetPlayerPawn` 0)) (!= (`GameplayStatics.GetObjectClass` OtherComp) "/Script/Engine.BoxComponent"))
    (set `self.playerClose?` true)
    (bind _asthird_person_character (cast `/Game/UltraMap/Mannequin/Character/ThirdPersonCharacter` OtherActor)
      (:`then`
        (set `/Game/UltraMap/Mannequin/Character/ThirdPersonCharacter.inRangeActor` self _asthird_person_character))
      (:`CastFailed`
        (`KismetSystemLibrary.PrintString` "Cast to ThirdPersonCharacter failed. Did you change the player pawn/character?")))))

(event `self.Box.OnComponentEndOverlap`
  (params (OverlappedComponent :type "PrimitiveComponent Object Reference") (OtherActor :type "Actor Object Reference") (OtherComp :type "PrimitiveComponent Object Reference") (OtherBodyIndex :type Integer))
  ;[1 1 1] Removes the actor placed on the stand from memory
  (if (and (== OtherActor (`GameplayStatics.GetPlayerPawn` 0)) (!= (`GameplayStatics.GetObjectClass` OtherComp) "/Script/Engine.BoxComponent"))
    (set `self.playerClose?` false)
    (bind _asthird_person_character (cast `/Game/UltraMap/Mannequin/Character/ThirdPersonCharacter` OtherActor)
      (:`then`
        (set `/Game/UltraMap/Mannequin/Character/ThirdPersonCharacter.inRangeActor` null _asthird_person_character))
      (:`CastFailed`
        (`KismetSystemLibrary.PrintString` "Cast to ThirdPersonCharacter failed. Did you change the player pawn/character?")))))

(fn `UserConstructionScript`)